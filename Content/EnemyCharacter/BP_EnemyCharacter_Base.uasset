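; BP_EnemyCharacter_Base is a base enemy character Blueprint that handles the death sequence in OnEnemyDied.
; On death it pauses mesh animation, disables capsule collision and drives a Fading parameter on a dynamic DeadMaterial instance through a timeline.
; After a short delay it destroys the equipped weapon from EnemyCombatComponent and then itself, both only when that weapon is valid.
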(event `self.ReceiveBeginPlay`)

(event `/Game/EnemyCharacter/BPI_Enemy_Death.OnEnemyDied`
  (bind _returnvalue (`PawnCombatComponent.GetCharacterCurrentEquippedWeapon` (`self.EnemyCombatComponent`)))
  (`|ExecutionSequence`
    (:`then_0`
      (set `SkeletalMeshComponent.bPauseAnims` true (`self.Mesh`))
      (`PrimitiveComponent.SetCollisionEnabled` (`self.CapsuleComponent`) "NoCollision"))
    (:`then_1`
      (bind _returnvalue_2 (`PrimitiveComponent.CreateDynamicMaterialInstance` (`self.Mesh`) 0 (`self.DeadMaterial`) "None"))
      (bind (_direction _newtrack_0) (`Timeline|Timeline`)
        (:`Update`
          (`MaterialInstanceDynamic.SetScalarParameterValue` _returnvalue_2 "Fading" _newtrack_0))))
    (:`then_2`
      (`KismetSystemLibrary.Delay` 2.0)
      (`/Engine/EditorBlueprintResources/StandardMacros.IsValid` _returnvalue
        (:`Is Valid`
          (`self.K2_DestroyActor` _returnvalue)
          (`self.K2_DestroyActor`))))))

(fn `UserConstructionScript`)