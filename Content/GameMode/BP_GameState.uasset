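; BP_GameState tracks how many enemies remain and triggers victory when all are dead.
; On BeginPlay it counts the BP_Samurai actors in the level and binds CheckAllDied to the HasEnemyDied event.
; Each death decrements the count; at zero it spawns a BP_GoToMap actor targeting the "Start" level, pauses the game, switches to UI-only input with a cursor, and shows WBP_Victory.
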(event `self.ReceiveBeginPlay`
  (add `self.HasEnemyDied` (delegate `CheckAllDied`))
  (bind _outactors (`GameplayStatics.GetAllActorsOfClass` "/Game/EnemyCharacter/Person/BP_Samurai.BP_Samurai_C"))
  (set `self.CurrentEnemyNum` (`KismetArrayLibrary.Array_Length` _outactors)))

(event `CheckAllDied`
  (bind _returnvalue (`GameplayStatics.GetPlayerController` 0))
  (`/Engine/EditorBlueprintResources/StandardMacros.DecrementInt` (`self.CurrentEnemyNum`)
    (:`  `
      (if (== (`self.CurrentEnemyNum`) 0)
        (`|SpawnActorFromClass` "/Game/Maps/Scene/BP_GoToMap.BP_GoToMap_C" (`KismetMathLibrary.MakeTransform` (1500.0 1500.0 0.0) (struct :`Yaw` 180.0)) "Undefined" "MultiplyWithRoot" null "Start" null)
        (`GameplayStatics.SetGamePaused` true)
        (`WidgetBlueprintLibrary.SetInputMode_UIOnlyEx` _returnvalue null)
        (set `PlayerController.bShowMouseCursor` true _returnvalue)
        (bind _returnvalue_2 (`|CreateWidget` "/Game/Widget/HeroWidget/WBP_Victory.WBP_Victory_C" (`GameplayStatics.GetPlayerController` 0)))
        (`UserWidget.AddToViewport` _returnvalue_2 0)))))

(fn `UserConstructionScript`)