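; BP_HeroCharacter is the player hero character, handling a walk speed toggle, a death camera and the pause menu.
; Left Ctrl flip-flops the movement component's max walk speed between slow and faster values.
; DeadCameraSwitch swaps the follow camera for the death camera, which a timeline offsets backward along its forward vector.
; Escape pauses the game, switches to UI-only input with a cursor, and displays WBP_ESC.
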(event `Key|LeftControl`
  (params (Key :type "Key Structure"))
  (bind _charactermovement (`self.CharacterMovement`))
  (:`Pressed`
    (`/Engine/EditorBlueprintResources/StandardMacros.FlipFlop`
      (:`A`
        (set `CharacterMovementComponent.MaxWalkSpeed` 200.0 _charactermovement))
      (:`B`
        (set `CharacterMovementComponent.MaxWalkSpeed` 400.0 _charactermovement)))))

(event `DeadCameraSwitch`
  (bind _deathcamera (`self.DeathCamera`))
  (`ActorComponent.SetActive` (`self.FollowCamera`) false false)
  (`ActorComponent.SetActive` _deathcamera true false)
  (bind (_direction _newtrack_0) (`Timeline|Timeline`)
    (:`Update`
      (`SceneComponent.K2_SetRelativeLocation` (`self.DeathCamera`) (* (* (`SceneComponent.GetForwardVector` _deathcamera) -1.0) _newtrack_0) false false))))

(event `Key|Escape`
  (params (Key :type "Key Structure"))
  (bind _returnvalue (`GameplayStatics.GetPlayerController` 0))
  (:`Pressed`
    (`GameplayStatics.SetGamePaused` true)
    (`WidgetBlueprintLibrary.SetInputMode_UIOnlyEx` _returnvalue null)
    (set `PlayerController.bShowMouseCursor` true _returnvalue)
    (bind _returnvalue_2 (`|CreateWidget` "/Game/Widget/HeroWidget/WBP_ESC.WBP_ESC_C" (`GameplayStatics.GetPlayerController` 0)))
    (`UserWidget.AddToViewport` _returnvalue_2 0)))

(fn `UserConstructionScript`)