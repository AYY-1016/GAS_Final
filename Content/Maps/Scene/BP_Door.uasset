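; BP_Door is an interactive hinged door that the player toggles with the F key while the hero stands in its trigger box.
; Box overlap shows a prompt widget, enables input and opens a gate; leaving undoes these and swings the door shut.
; A FlipFlop plays or reverses a timeline driving door yaw, with sound on opening.
; A dot product of door and player forward vectors picks the swing direction.
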(event `Key|F`
  (params (Key :type "Key Structure"))
  (:`Pressed`
    (`/Engine/EditorBlueprintResources/StandardMacros.Gate` true :!label _label
      (:`Exit`
        (`/Engine/EditorBlueprintResources/StandardMacros.FlipFlop`
          (:`A`
            (`self.JudgeOpenDoorDirection`)
            (`GameplayStatics.PlaySoundAtLocation` "/Game/Free_Sounds_Pack/wav/Door_Open_4-1.Door_Open_4-1" (`self.K2_GetActorLocation`) (struct) 1.0 1.0 0.0 null null null null)
            (bind (_direction _rotation) (`Timeline|OpenOrCloseDoor` :!label _label_2)
              (:`Update`
                (`SceneComponent.K2_SetRelativeRotation` (`self.Door`) (`KismetMathLibrary.MakeRotator` 0.0 0.0 (* (`KismetMathLibrary.Lerp` 0.0 75.0 _rotation) (`self.Direction`))) false false))))
          (:`B`
            (goto _label_2 :!via `Reverse`)))))))

(event `self.Box.OnComponentBeginOverlap`
  (params (OverlappedComponent :type "PrimitiveComponent Object Reference") (OtherActor :type "Actor Object Reference") (OtherComp :type "PrimitiveComponent Object Reference") (OtherBodyIndex :type Integer) (bFromSweep :type Boolean) (SweepResult :type "HitResult Structure (by ref)"))
  (cast `/Game/PlayerCharacter/BP_HeroCharacter` OtherActor)
  (`SceneComponent.SetVisibility` (`self.Widget`) true false)
  (`self.EnableInput` (`GameplayStatics.GetPlayerController` 0))
  (goto _label :!via `Open`))

(event `self.Box.OnComponentEndOverlap`
  (params (OverlappedComponent :type "PrimitiveComponent Object Reference") (OtherActor :type "Actor Object Reference") (OtherComp :type "PrimitiveComponent Object Reference") (OtherBodyIndex :type Integer))
  (cast `/Game/PlayerCharacter/BP_HeroCharacter` OtherActor)
  (`SceneComponent.SetVisibility` (`self.Widget`) false false)
  (`|ExecutionSequence`
    (:`then_0`
      (`self.DisableInput` (`GameplayStatics.GetPlayerController` 0))
      (goto _label :!via `Close`))
    (:`then_1`
      (goto _label_2 :!via `Reverse`))))

(fn `JudgeOpenDoorDirection`
  (if (< (`KismetMathLibrary.Dot_VectorVector` (`SceneComponent.GetForwardVector` (`self.Door`)) (`SceneComponent.GetForwardVector` (`Actor.RootComponent` (`GameplayStatics.GetPlayerCharacter` 0)))) 0.0)
    (set `self.Direction` -1)
    (else
      (set `self.Direction` 1))))

(fn `UserConstructionScript`)