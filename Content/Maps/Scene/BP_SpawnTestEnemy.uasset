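; BP_SpawnTestEnemy is a trigger actor that spawns a Bp_TestEnemy when F is pressed while the hero is inside its Box.
; Box overlap with BP_HeroCharacter enables input from player 0 and opens a gate; end overlap disables input and closes it.
; Each F press that passes the gate spawns one enemy at a random positive X/Y offset from the actor.
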(event `Key|F`
  (params (Key :type "Key Structure"))
  (bind _returnvalue (`KismetMathLibrary.RandomFloatInRange` 100.0 200.0))
  (:`Pressed`
    (`/Engine/EditorBlueprintResources/StandardMacros.Gate` true :!label _label
      (:`Exit`
        (`|SpawnActorFromClass` "/Game/EnemyCharacter/TestEnemy/Bp_TestEnemy.Bp_TestEnemy_C" (`KismetMathLibrary.MakeTransform` (+ (`self.K2_GetActorLocation`) (`KismetMathLibrary.MakeVector` _returnvalue _returnvalue))) "Undefined" "MultiplyWithRoot" null null)))))

(event `self.Box.OnComponentBeginOverlap`
  (params (OverlappedComponent :type "PrimitiveComponent Object Reference") (OtherActor :type "Actor Object Reference") (OtherComp :type "PrimitiveComponent Object Reference") (OtherBodyIndex :type Integer) (bFromSweep :type Boolean) (SweepResult :type "HitResult Structure (by ref)"))
  (cast `/Game/PlayerCharacter/BP_HeroCharacter` OtherActor)
  (`self.EnableInput` (`GameplayStatics.GetPlayerController` 0))
  (goto _label :!via `Open`))

(event `self.Box.OnComponentEndOverlap`
  (params (OverlappedComponent :type "PrimitiveComponent Object Reference") (OtherActor :type "Actor Object Reference") (OtherComp :type "PrimitiveComponent Object Reference") (OtherBodyIndex :type Integer))
  (cast `/Game/PlayerCharacter/BP_HeroCharacter` OtherActor)
  (`self.DisableInput` (`GameplayStatics.GetPlayerController` 0))
  (goto _label :!via `Close`))

(fn `UserConstructionScript`)